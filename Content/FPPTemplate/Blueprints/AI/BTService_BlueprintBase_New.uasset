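; Behavior tree service that snaps the controlled pawn between four MoveActor1 marker actors in a repeating cycle.
; On activation it finds the markers and stores those numbered 1, 2, 4 and 5.
; Its tick reads the seconds counter on BP_FPPT_HUD and advances a wrapping index once at least two seconds pass.
; A MultiGate, using that index as start index, selects the marker for an unswept SetActorLocation.
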(event EventReceiveActivationAI
  (params (OwnerController :type AI%20Controller%20Object%20Reference) (ControlledPawn :type Pawn%20Object%20Reference))
  (bind _outactors (Actor|GetAllActorsOfClass "/Game/FPPTemplate/Blueprints/AI/MoveAct/MoveActor1.MoveActor1_C"))
  (for _array_element _outactors
    (switch int (Variables|/Game/FPPTemplate/Blueprints/AI/MoveAct/MoveActor1.MoveActor1_C|GetNum _array_element)
      (:1
        (Variables|Default|SetNewVar_1 _array_element))
      (:2
        (Variables|Default|SetNewVar_2 _array_element))
      (:4
        (Variables|Default|SetNewVar_4 _array_element))
      (:5
        (Variables|Default|SetNewVar_5 _array_element)))))

(event EventReceiveTickAI
  (params (OwnerController :type AI%20Controller%20Object%20Reference) (ControlledPawn :type Pawn%20Object%20Reference) (DeltaSeconds :type Float%20%28single-precision%29))
  (Variables|Default|SetPawn ControlledPawn)
  (bind _asbp_fppt_hud (Utilities|Casting|CastToBP_FPPT_HUD (HUD|GetHUD (Game|GetPlayerController 0))))
  (if (>= (- (Variables|/Game/FPPTemplate/Blueprints/Game/BP_FPPT_HUD.BP_FPPT_HUD_C|GetSecond _asbp_fppt_hud) (Variables|Default|GetPasTime)) 2)
    (Variables|Default|SetPasTime (Variables|/Game/FPPTemplate/Blueprints/Game/BP_FPPT_HUD.BP_FPPT_HUD_C|GetSecond _asbp_fppt_hud))
    (CallFunction|CalCount)))

(fn CalCount
  (bind _output_get (Variables|Default|SetCount (+ (Variables|Default|GetCount) 1)))
  (if (== _output_get 4)
    (bind _output_get_2 (Variables|Default|SetCount 0))
    (CallFunction|Moveto _output_get_2)
    (else
      (CallFunction|Moveto _output_get))))

(fn Moveto
  (params (NewParam :type Integer))
  (bind _pawn (Variables|Default|GetPawn))
  (Utilities|FlowControl|MultiGate false false NewParam
    (:Out%200
      (Transformation|SetActorLocation _pawn (Transformation|GetActorLocation (Variables|Default|GetNewVar_1)) false false))
    (:Out%201
      (Transformation|SetActorLocation _pawn (Transformation|GetActorLocation (Variables|Default|GetNewVar_2)) false false))
    (:Out%202
      (Transformation|SetActorLocation _pawn (Transformation|GetActorLocation (Variables|Default|GetNewVar_4)) false false))
    (:Out%203
      (Transformation|SetActorLocation _pawn (Transformation|GetActorLocation (Variables|Default|GetNewVar_5)) false false))))