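; Monster actor that teleports between five MoveActor1 waypoints on a looping timer, changing only its X and Y.
; BeginPlay caches waypoints by their Num and registers the monster with BP_FPPT_HUD.
; StartTime starts the timer, whose tick advances a wrapping Count that a MultiGate uses as start index to pick the waypoint.
; ResetAll clears the timer and resets Count; DetectPlayer is called each tick but is empty.
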(event Custom|StartTime
  (bind _returnvalue (Utilities|Time|SetTimerbyEvent (delegate Custom|UpdateLocation) 2.0 true))
  (Variables|Default|SetTimeHandle _returnvalue))

(event Custom|UpdateLocation
  (CallFunction|CalCount)
  (CallFunction|Moveto)
  (CallFunction|DetectPlayer))

(event EventBeginPlay
  (Utilities|FlowControl|Sequence
    (:then_0
      (bind _outactors (Actor|GetAllActorsOfClass "/Game/FPPTemplate/Blueprints/AI/MoveAct/MoveActor1.MoveActor1_C"))
      (for _array_element _outactors
        (switch int (Variables|/Game/FPPTemplate/Blueprints/AI/MoveAct/MoveActor1.MoveActor1_C|GetNum _array_element)
          (:1
            (Variables|Default|SetNewVar_1 _array_element))
          (:2
            (Variables|Default|SetNewVar_2 _array_element))
          (:4
            (Variables|Default|SetNewVar_4 _array_element))
          (:5
            (Variables|Default|SetNewVar_5 _array_element))
          (:6
            (Variables|Default|SetNewVar_6 _array_element)))))
    (:then_1
      (bind _asbp_fppt_hud (Utilities|Casting|CastToBP_FPPT_HUD (HUD|GetHUD (Game|GetPlayerController 0))))
      (Variables|/Game/FPPTemplate/Blueprints/Game/BP_FPPT_HUD.BP_FPPT_HUD_C|SetMonster _asbp_fppt_hud self))))

(fn ConstructionScript)

(fn Moveto
  (bind _newvar_5 (Variables|Default|GetNewVar_5))
  (bind _newvar_1 (Variables|Default|GetNewVar_1))
  (bind _newvar_6 (Variables|Default|GetNewVar_6))
  (bind _newvar_2 (Variables|Default|GetNewVar_2))
  (bind _newvar_4 (Variables|Default|GetNewVar_4))
  (bind _returnvalue (Transformation|GetActorLocation _newvar_6))
  (bind _returnvalue_2 (Transformation|GetActorLocation _newvar_4))
  (bind _returnvalue_3 (Transformation|GetActorLocation _newvar_5))
  (bind _returnvalue_4 (Transformation|GetActorLocation _newvar_1))
  (bind _returnvalue_5 (Transformation|GetActorLocation _newvar_2))
  (Utilities|FlowControl|MultiGate false false (Variables|Default|GetCount)
    (:Out%200
      (Transformation|SetActorLocation (Math|Vector|MakeVector (.x _returnvalue_4) (.y _returnvalue_4) 0.0) false false))
    (:Out%201
      (Transformation|SetActorLocation (Math|Vector|MakeVector (.x _returnvalue_5) (.y _returnvalue_5) 0.0) false false))
    (:Out%202
      (Transformation|SetActorLocation (Math|Vector|MakeVector (.x _returnvalue_2) (.y _returnvalue_2) 0.0) false false))
    (:Out%203
      (Transformation|SetActorLocation (Math|Vector|MakeVector (.x _returnvalue_3) (.y _returnvalue_3) 0.0) false false))
    (:Out%204
      (Transformation|SetActorLocation (Math|Vector|MakeVector (.x _returnvalue) (.y _returnvalue) 0.0) false false))))

(fn CalCount
  (bind _output_get (Variables|Default|SetCount (+ (Variables|Default|GetCount) 1)))
  (if (== _output_get 5)
    (Variables|Default|SetCount 0)))

(fn DetectPlayer)

(fn ResetAll
  (Utilities|Time|ClearandInvalidateTimerbyHandle (Variables|Default|GetTimeHandle))
  (Variables|Default|SetCount -1))