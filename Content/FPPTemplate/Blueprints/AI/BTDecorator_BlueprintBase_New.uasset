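; A Behavior Tree decorator that tracks elapsed seconds for AI, using the Second counter on the player's BP_FPPT_HUD.
; When that counter is at least one ahead of the PasTime blackboard value, it writes the current second into PasTime.
; Both branches return true, so once the HUD cast succeeds the check updates the timestamp without blocking execution.
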(fn PerformConditionCheckAI
  (params (OwnerController :type AI%20Controller%20Object%20Reference) (ControlledPawn :type Pawn%20Object%20Reference))
  (bind _pastime (Variables|Default|GetPasTime))
  (bind _asbp_fppt_hud (Utilities|Casting|CastToBP_FPPT_HUD (HUD|GetHUD (Game|GetPlayerController 0))))
  (if (>= (- (Variables|/Game/FPPTemplate/Blueprints/Game/BP_FPPT_HUD.BP_FPPT_HUD_C|GetSecond _asbp_fppt_hud) (Class|BTFunctionLibrary|GetBlackboardValueasInt _pastime)) 1)
    (Class|BTFunctionLibrary|SetBlackboardValueasInt _pastime (Variables|/Game/FPPTemplate/Blueprints/Game/BP_FPPT_HUD.BP_FPPT_HUD_C|GetSecond _asbp_fppt_hud))
    (return true)
    (else
      (return true))))