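; First-person template HUD that shows a running clock, a small Bokeh texture drawn from screen center, and temporary object text.
; A looping one-second timer increments a counter and pushes it to the clock widget.
; ShowTextUI finds text by scanning data table rows for a matching object name, then displays it in a widget removed by a five-second timer.
; A name comparison decides whether an existing text widget is kept or replaced.
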(event Custom|OnUpdateTime
  (bind _output_get (Variables|Default|SetSecond (+ (Variables|Default|GetSecond) 1)))
  (Default|UpdateClock (Variables|Default|GetClockWbp) _output_get))

(event Custom|RemoveTextWbp
  (Variables|Default|SetTextHandle "")
  (Widget|RemovefromParent (stale Custom|ShowTextUI _output_get_2))
  (Variables|Default|SetTextWbp 0))

(event Custom|ShowTextUI
  (params (objectName :type String))
  (if (Utilities|Enum|Equal(Enum) objectName (Variables|Default|GetObjectName))
    (Utilities|IsValid (Variables|Default|GetTextWbp)
      (:Is%20Valid
        (Development|PrintString objectName))
      (:Is%20Not%20Valid
        (bind _output_get (Variables|Default|SetObjectName objectName :!label _label))
        (bind _newparam (CallFunction|FindDatatableObjectname _output_get))
        (bind _returnvalue (UserInterface|CreateWidget "/Game/FPPTemplate/Blueprints/UI/Text_WBP.Text_WBP_C"))
        (Default|SetShowText _returnvalue _newparam)
        (bind _output_get_2 (Variables|Default|SetTextWbp _returnvalue))
        (UserInterface|Viewport|AddtoViewport _output_get_2 0)
        (bind _returnvalue_2 (Utilities|Time|SetTimerbyEvent (delegate Custom|RemoveTextWbp) 5.0))
        (Variables|Default|SetTextHandle _returnvalue_2)))
    (else
      (Utilities|IsValid (Variables|Default|GetTextWbp)
        (:Is%20Valid
          (CallFunction|RemoveTextWbp)
          (goto _label))
        (:Is%20Not%20Valid
          (goto _label))))))

(event EventBeginPlay
  (Utilities|Time|SetTimerbyEvent (delegate Custom|OnUpdateTime) 1.0 true)
  (bind _returnvalue (UserInterface|CreateWidget "/Game/FPPTemplate/Blueprints/UI/Clock_WBP.Clock_WBP_C"))
  (bind _output_get (Variables|Default|SetClockWbp _returnvalue))
  (UserInterface|Viewport|AddtoViewport _output_get 0))

(event Collision|EventActorBeginOverlap
  (params (OtherActor :type Actor%20Object%20Reference)))

(event EventTick
  (params (DeltaSeconds :type Float%20%28single-precision%29)))

(event EventDrawHUD
  (params (SizeX :type Integer) (SizeY :type Integer))
  (Class|HUD|DrawTextureSimple "/Engine/Engine_MI_Shaders/Textures/Bokeh.Bokeh" (Math|Conversions|ToFloat(Integer) (/ SizeX 2)) (Math|Conversions|ToFloat(Integer) (/ SizeY 2)) 0.3 false))

(fn ConstructionScript)

(fn FindDatatableObjectname
  (params (ObjectName :type String))
  (bind _datatable (Variables|Default|GetDataTable))
  (bind _outrownames (DataTable|GetDataTableRowNames _datatable))
  (for _array_element _outrownames
    (bind _returnvalue (Utilities|GetDataTableRow _datatable _array_element)
      (:then
        (if (Utilities|Enum|Equal(Enum) ObjectName (.ObjectName (Utilities|Struct|BreakNewUserDefinedStruct _returnvalue)))
          (return (.Text (Utilities|Struct|BreakNewUserDefinedStruct _returnvalue))))))))