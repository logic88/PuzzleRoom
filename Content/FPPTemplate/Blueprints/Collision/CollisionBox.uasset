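; CollisionBox is a trigger actor that tracks which actors are inside its Box component and reports a game-over condition through debug prints.
; Begin and end overlap events print the other actor's name with an In or Out tag and add or remove that actor in the NewVar collection.
; When an entry brings the collection to two or more actors, it prints "GameOver", with no further game-ending logic.
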(event OnComponentBeginOverlap(Box)
  (params (OverlappedComponent :type Primitive%20Component%20Object%20Reference) (OtherActor :type Actor%20Object%20Reference) (OtherComp :type Primitive%20Component%20Object%20Reference) (OtherBodyIndex :type Integer) (bFromSweep :type Boolean) (SweepResult :type Hit%20Result%20Structure%20%28by%20ref%29))
  (bind _newvar (Variables|Default|GetNewVar))
  (Development|PrintString (Utilities|String|Append (Utilities|String|Append (Utilities|String|Append (Utilities|GetObjectName OtherActor) ":") (Utilities|GetObjectName self)) ":In") true true "(R=0.000000,G=0.660000,B=1.000000,A=1.000000)" 1.0)
  (Utilities|Array|Add _newvar OtherActor)
  (if (>= (Utilities|Array|Length _newvar) 2)
    (Development|PrintString "GameOver")))

(event OnComponentEndOverlap(Box)
  (params (OverlappedComponent :type Primitive%20Component%20Object%20Reference) (OtherActor :type Actor%20Object%20Reference) (OtherComp :type Primitive%20Component%20Object%20Reference) (OtherBodyIndex :type Integer))
  (Development|PrintString (Utilities|String|Append (Utilities|String|Append (Utilities|String|Append (Utilities|GetObjectName OtherActor) ":") (Utilities|GetObjectName self)) ":Out") true true "(R=0.000000,G=0.660000,B=1.000000,A=1.000000)" 1.0)
  (Utilities|Array|RemoveItem (Variables|Default|GetNewVar) OtherActor))

(event EventBeginPlay)

(event Collision|EventActorBeginOverlap
  (params (OtherActor :type Actor%20Object%20Reference)))

(event EventTick
  (params (DeltaSeconds :type Float%20%28single-precision%29)))

(fn ConstructionScript)